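; Blink component that simulates eye hydration and forced blinking, and tracks whether its owner can see.
; A looping one-second timer drains hydration when it is below maximum and triggers a blink at zero.
; Blink is latched by a DoOnce and adds an UnrealmotionG widget holding a component reference, while Endblink refills hydration and resets the latch.
; Tick clears CanSee during blinks or in darkness without a flashlight.
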(event `self.ReceiveBeginPlay`
  (`KismetSystemLibrary.K2_SetTimerDelegate` (delegate `Hydration loop`) 1.0 true))

(event `Hydration loop`
  ;[1 1 1] Eye Hydrationlevel drain loop
  (if (== (`self.Eye Hydrationmax`) (`self.Eye Hydration`))
    (`/Engine/EditorBlueprintResources/StandardMacros.DoOnce` false :!label _label
      (:`Completed`
        (`KismetSystemLibrary.Delay` (`self.Hydration Delay`))))
    (else
      (`|ExecutionSequence`
        (:`then_0`
          (goto _label :!via `Reset`))
        (:`then_1`
          (bind _output_get (set `self.Eye Hydration` (- (`self.Eye Hydration`) (`self.Eye Hydration Drain`))))
          (if (<= _output_get 0.0)
            (`self.Blink`)))))))

(event `Blink`
  ;[1 1 1] Blinking
  (`/Engine/EditorBlueprintResources/StandardMacros.DoOnce` false :!label _label_2
    (:`Completed`
      (set `self.Blinking` true)
      (bind _returnvalue (`|CreateWidget` "/Game/Services/Blueprints/Widgets/UnrealmotionG.UnrealmotionG_C"))
      (set `/Game/Services/Blueprints/Widgets/UnrealmotionG.Blinkcomponent` self _returnvalue)
      (`UserWidget.AddToPlayerScreen` _returnvalue 0))))

(event `End blink`
  ;[1 1 1] Blinking
  (set `self.Blinking` false)
  (set `self.Eye Hydration` (`self.Eye Hydrationmax`))
  (goto _label_2 :!via `Reset`))

(event `self.ReceiveTick`
  (params (DeltaSeconds :type "Float (single-precision)"))
  ;[1 1 1] Set can see
  (set `self.CanSee` (not (or (and (`self.Dark`) (not (`self.Flashlight`))) (`self.Blinking`)))))