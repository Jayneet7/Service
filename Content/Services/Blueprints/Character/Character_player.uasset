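; Player character Blueprint that handles first-person style movement, look and a blink ability.
; Walk and Strafe axes add movement along the actor's forward and right vectors.
; Pitch and Yaw feed controller rotation, with Pitch also copying control rotation onto the camera's world rotation.
; The Blinking action calls Blink on a separate BlinkComponent, which holds the ability's logic.
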(event `InputAxis|Walk`
  (params (AxisValue :type "Float (single-precision)"))
  (`self.AddMovementInput` (`self.GetActorForwardVector`) AxisValue))

(event `InputAxis|Pitch`
  (params (AxisValue :type "Float (single-precision)"))
  (`self.AddControllerPitchInput` AxisValue)
  (`SceneComponent.K2_SetWorldRotation` (`self.Camera`) (`self.GetControlRotation`) false false))

(event `InputAxis|Strafe`
  (params (AxisValue :type "Float (single-precision)"))
  (`self.AddMovementInput` (`self.GetActorRightVector`) AxisValue))

(event `InputAxis|Yaw`
  (params (AxisValue :type "Float (single-precision)"))
  (`self.AddControllerYawInput` AxisValue))

(event `InputAction|Blinking`
  (params (Key :type "Key Structure"))
  (:`Pressed`
    (`/Game/Services/Blueprints/Character/BlinkComponent.Blink` (`self.BlinkComponent`))))

(fn `UserConstructionScript`)