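; Behavior tree service that gives an enemy AI a player target through sight checks and short-term memory.
; Without a current or remembered target, it loops through player characters for the closest one passing a view-cone angle test and line-of-sight trace.
; Each tick revalidates the target, writing it to the blackboard via TargetMemory.
; A retriggerable delay forgets lost targets, and searching waits until then.
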(event `self.ReceiveTickAI`
  (params (OwnerController :type "AIController Object Reference") (ControlledPawn :type "Pawn Object Reference") (DeltaSeconds :type "Float (single-precision)"))
  (set `self.Enemy Pawn` ControlledPawn)
  (`/Engine/EditorBlueprintResources/StandardMacros.IsValid` (`self.Target Char`)
    (:`Is Valid`
      (bind _targetisvalid (`self.Validate target` (`self.Target Char`)))
      (if _targetisvalid
        (set `self.Target Memory` (`self.Target Char`))
        (`self.Target memeory timer`)
        (`BTFunctionLibrary.SetBlackboardValueAsObject` (`self.TargetKey`) (`self.Target Memory`) :!label _label)
        (else
          (set `self.Target Char` null))))
    (:`Is Not Valid`
      (`/Engine/EditorBlueprintResources/StandardMacros.IsValid` (`self.Target Memory`)
        (:`Is Valid`
          (goto _label))
        (:`Is Not Valid`
          (`self.Find Target`))))))

(event `Find Target`
  (bind _enemy_pawn (`self.Enemy Pawn`))
  (bind _target_char (`self.Target Char`))
  ;[1 1 1] Loop through player characters
  (for _index (range (+ (`self.Maxplayer`) 1))
    (bind _returnvalue (`GameplayStatics.GetPlayerCharacter` _index))
    (`/Engine/EditorBlueprintResources/StandardMacros.IsValid` _returnvalue
      (:`Is Valid`
        (`/Engine/EditorBlueprintResources/StandardMacros.IsValid` (`self.Target Char`)
          (:`Is Valid`
            (bind _returnvalue_2 (select `bool` (>= (`Actor.GetDistanceTo` _returnvalue _enemy_pawn) (`Actor.GetDistanceTo` _enemy_pawn _target_char)) :`false` _returnvalue :`true` _target_char))
            ;[1 1 1] Find Closest target
            (bind _targetisvalid (`self.Validate target` _returnvalue_2))
            (if _targetisvalid
              (set `self.Target Char` _returnvalue_2)))
          (:`Is Not Valid`
            ;[1 1 1] Set target to valid character
            (bind _targetisvalid_2 (`self.Validate target` _returnvalue))
            (if _targetisvalid_2
              (set `self.Target Char` _returnvalue))))))))

(event `Target memeory timer`
  ;[1 1 1] Timer to forget target
  (`KismetSystemLibrary.RetriggerableDelay` (`self.Memorytime`))
  (set `self.Target Memory` null))

(fn `Validate target`
  (params (TestChar :type "Character Object Reference"))
  (returns (TargetIsvalid :type Boolean))
  (locals (Isvalid :type Boolean) (TempChar :type "Character Object Reference"))
  (bind _enemy_pawn (`self.Enemy Pawn`))
  (bind _enemy_pawn_2 (`self.Enemy Pawn`))
  (set `local.TempChar` TestChar)
  (set `local.Isvalid` false)
  (if (<= (`KismetMathLibrary.DegAcos` (`KismetMathLibrary.Dot_VectorVector` (`Actor.GetActorForwardVector` _enemy_pawn) (`KismetMathLibrary.GetForwardVector` (`KismetMathLibrary.FindLookAtRotation` (`Actor.K2_GetActorLocation` _enemy_pawn) (`Actor.K2_GetActorLocation` (`local.TempChar`)))))) (`self.HaldVision`))
    ;[1 1 1] Does enemy have line of seight
    (bind _outhit (`KismetSystemLibrary.LineTraceSingle` (+ (`Actor.K2_GetActorLocation` _enemy_pawn_2) (`self.HeighOffset`)) (`Actor.K2_GetActorLocation` (`local.TempChar`)) "TraceTypeQuery2" false (`|MakeArray` _enemy_pawn_2 :!type "Actor Object Reference") "ForDuration"))
    (if (== (`.HitActor` (`GameplayStatics.BreakHitResult` _outhit)) (`local.TempChar`))
      (set `local.Isvalid` true))
    (return (`local.Isvalid`))
    (else
      (return (`local.Isvalid`)))))