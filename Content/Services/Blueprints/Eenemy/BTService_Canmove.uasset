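; Behavior tree service that writes a Canmove blackboard bool for an enemy, apparently meant to freeze it while players watch.
; Each tick it checks every player's BlinkComponent CanSee and a zero-degree facing threshold.
; Passing players get four debug-drawn Camera-channel traces between offset points on both characters.
; The hit check that would clear Canmove is disconnected, so the key is always written true.
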(event `self.ReceiveTickAI`
  (params (OwnerController :type "AIController Object Reference") (ControlledPawn :type "Pawn Object Reference") (DeltaSeconds :type "Float (single-precision)"))
  (bind _tempchar (`self.Tempchar`))
  (bind _enemypawn (`self.Enemypawn`))
  (bind _ascharacter (cast `Character` _enemypawn :!pure true))
  (set `self.Enemypawn` ControlledPawn)
  (set `self.Canmove` true)
  ;[1 1 1] For each charecter check if they can see if enemy is in field of view
  (for _index (range (+ (`self.Maxplayers`) 1))
    (bind _returnvalue (`GameplayStatics.GetPlayerCharacter` _index))
    (set `self.Tempchar` _returnvalue)
    (`/Engine/EditorBlueprintResources/StandardMacros.IsValid` _returnvalue
      (:`Is Valid`
        (bind _returnvalue_2 (`Actor.GetComponentByClass` _returnvalue "/Game/Services/Blueprints/Character/BlinkComponent.BlinkComponent_C"))
        (`/Engine/EditorBlueprintResources/StandardMacros.IsValid` _returnvalue_2
          (:`Is Valid`
            (if (and (`/Game/Services/Blueprints/Character/BlinkComponent.CanSee` _returnvalue_2) (<= (`KismetMathLibrary.DegAcos` (`KismetMathLibrary.Dot_VectorVector` (`Actor.GetActorForwardVector` _returnvalue) (`KismetMathLibrary.GetForwardVector` (`KismetMathLibrary.FindLookAtRotation` (`Actor.K2_GetActorLocation` _returnvalue) (`Actor.K2_GetActorLocation` (`self.Enemypawn`)))))) 0.0))
              ;[1 1 1] sides of enemy and charecter for line of seight
              (for _index_2 (range 4)
                (bind _outhit (`KismetSystemLibrary.LineTraceSingle` (+ (`Actor.K2_GetActorLocation` _tempchar) (`|GetArrayItem` (`|MakeArray` (`self.NewMacro_0` _tempchar 1.0 1.0) (`self.NewMacro_0` _tempchar -1.0 1.0) (`self.NewMacro_0` _tempchar 1.0 -1.0) (`self.NewMacro_0` _tempchar -1.0 -1.0)) _index_2)) (+ (`Actor.K2_GetActorLocation` _enemypawn) (`|GetArrayItem` (`|MakeArray` (`self.NewMacro_0` _ascharacter 1.0 1.0) (`self.NewMacro_0` _ascharacter -1.0 1.0) (`self.NewMacro_0` _ascharacter 1.0 -1.0) (`self.NewMacro_0` _ascharacter -1.0 -1.0)) _index_2)) "TraceTypeQuery2" false (`|MakeArray` _tempchar :!type "Actor Object Reference") "ForDuration" false (struct :`R` 1.0 :`G` 0.367106 :`B` 0.186432 :`A` 1.0) (struct :`R` 0.135354 :`G` 0.224407 :`B` 1.0 :`A` 1.0))))))))))
  (`BTFunctionLibrary.SetBlackboardValueAsBool` (`self.CanmoveKey`) (`self.Canmove`)))